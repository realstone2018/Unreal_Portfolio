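; Player controller Blueprint that owns the game's UI: HUD, stage timer, result screen and respawn countdown.
; BeginPlay creates the HUD and caches its stage timer widget, which OnTimerStart runs using the clear time from PTGameModeBase.
; Clear and game-over events share one result-widget path, differing only by the IsClear flag.
; OnPlayerRespawn creates a respawn widget timed by the game mode's remaining respawn time.
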(event `self.ReceiveBeginPlay`
  ;[1 1 1] Init HUD
  (bind _returnvalue (`|CreateWidget` "/Game/Project2/UI/WBP_HUD.WBP_HUD_C"))
  (`UserWidget.AddToViewport` _returnvalue 0)
  (set `self.HUD` _returnvalue)
  (set `self.WBPStageTimer` (`/Game/Project2/UI/WBP_HUD.WidgetStageTimer` _returnvalue)))

(event `self.K2_OnTimerStart`
  ;[1 1 1] StartTimer
  (bind _asptgame_mode_base (cast `PTGameModeBase` (`GameplayStatics.GetGameMode`)))
  (`/Game/Project2/UI/WBP_StageTimer.StartTimer` (`self.WBPStageTimer`) (`PTGameModeBase.StageClearTime` _asptgame_mode_base)))

(event `self.K2_OnGameClear`
  ;[1 1 1] Show Result
  (set `self.IsClear` true)
  (bind _returnvalue (`|CreateWidget` "/Game/Project2/UI/WBP_ResultWidget.WBP_ResultWidget_C" (`GameplayStatics.GetPlayerController` 0) :!label _label))
  (`UserWidget.AddToViewport` _returnvalue 0)
  (`/Game/Project2/UI/WBP_ResultWidget.SetResult` _returnvalue (`self.IsClear`)))

(event `self.K2_OnGameOver`
  ;[1 1 1] Show Result
  (set `self.IsClear` false)
  (goto _label))

(event `self.K2_OnPlayerRespawn`
  ;[1 1 1] Show Player Respawn Delay
  (bind _returnvalue (`|CreateWidget` "/Game/Project2/UI/WBP_PlayerReSpawn.WBP_PlayerReSpawn_C" (`GameplayStatics.GetPlayerController` 0)))
  (bind _output_get (set `self.WBPPlayerRespawn` _returnvalue))
  (`UserWidget.AddToViewport` _output_get 0)
  (bind _asptgame_mode_base (cast `PTGameModeBase` (`GameplayStatics.GetGameMode`)))
  (bind _returnvalue_2 (`PTGameModeBase.GetPlayerRespawnRemainTime` _asptgame_mode_base))
  (`/Game/Project2/UI/WBP_PlayerReSpawn.StartTimer` (`self.WBPPlayerRespawn`) _returnvalue_2))

(fn `UserConstructionScript`)